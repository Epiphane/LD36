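; FinalDoor is a door Blueprint that fires Trigger once every entry in its Indicators collection is on.
; Each Tick, until complete, it assumes success, then scans the indicators and clears IsComplete if any is off.
; It also calls SetState(false) on Result during this check.
; IsComplete then latches, so polling stops after the trigger.
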(event EventBeginPlay
  (|CallParentFunction))

(event Collision|EventActorBeginOverlap
  (params (OtherActor :type Actor%20Object%20Reference)))

(event EventTick
  (params (DeltaSeconds :type Float%20%28single-precision%29))
  (|CallParentFunction DeltaSeconds)
  (if (not (Variables|Default|GetIsComplete))
    (Variables|Default|SetIsComplete true)
    (for _array_element (Variables|Default|GetIndicators)
      (if (not (Variables|/Game/Blueprints/ActivatableLight.ActivatableLight_C|GetIsOn _array_element))
        (Variables|Default|SetIsComplete false)))
    (Default|SetState (Variables|Default|GetResult) false)
    (if (Variables|Default|GetIsComplete)
      (CallFunction|Trigger))))

(fn ConstructionScript
  (|CallParentFunction))