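; DeathCamera is a camera actor that becomes the player's view when the Explorer pawn dies.
; Each tick while the Explorer lives, it sits behind and above the pawn along the flattened control-rotation forward vector, aimed at the pawn.
; Once IsDead is set, it stops following and calls SetViewTargetWithBlend with a cubic blend every tick to make the camera's owner the view target.
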(event EventTick
  (params (DeltaSeconds :type Float%20%28single-precision%29))
  (bind _returnvalue (Game|Player|GetPlayerPawn 0))
  (bind _returnvalue_2 (Pawn|GetControlRotation _returnvalue :!class /Script/Engine.Pawn))
  (bind _returnvalue_3 (Math|Vector|GetForwardVector _returnvalue_2))
  (bind (_x _y) (Math|Vector|BreakVector _returnvalue_3))
  (bind _asexplorer (Utilities|Casting|CastToExplorer _returnvalue))
  (if (Variables|/Game/Blueprints/Explorer.Explorer_C|GetIsDead _asexplorer)
    (Game|Player|SetViewTargetwithBlend (Game|GetPlayerController 0) (Components|GetOwner (Variables|Default|GetCamera)) 0.0 "VTBlend_Cubic" 0.0 false)
    (else
      (Transformation|SetActorLocation (+ (- (Transformation|GetActorLocation _asexplorer) (* (Math|Vector|MakeVector _x _y 0.0) 1e+02)) "0, 0,200.000000") false false)
      (Transformation|SetActorRotation (Math|Rotator|FindLookatRotation (+ (- (Transformation|GetActorLocation _asexplorer) (* (Math|Vector|MakeVector _x _y 0.0) 1e+02)) "0, 0,200.000000") (Transformation|GetActorLocation _asexplorer))))))

(fn ConstructionScript)