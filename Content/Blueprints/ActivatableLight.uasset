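; ActivatableLight is an actor whose Cube mesh shows an on or off material to act as a switchable light.
; BeginPlay sets the Cube's material to OnMaterial or OffMaterial according to IsOn.
; The Trigger event flips IsOn and reuses the same branch to update the material.
; The file shows only material swaps, with no light component being changed.
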(event EventBeginPlay
  (if (stale EventTrigger _output_get)
    (Rendering|Material|SetMaterial (Variables|Default|GetCube) 0 (Variables|Default|GetOnMaterial))
    (else
      (Rendering|Material|SetMaterial (Variables|Default|GetCube) 0 (Variables|Default|GetOffMaterial)))))

(event EventTrigger
  (bind _output_get (Variables|Default|SetIsOn (not (Variables|Default|GetIsOn))))
  (if _output_get
    (Rendering|Material|SetMaterial (Variables|Default|GetCube) 0 (Variables|Default|GetOnMaterial))
    (else
      (Rendering|Material|SetMaterial (Variables|Default|GetCube) 0 (Variables|Default|GetOffMaterial)))))

(fn ConstructionScript
  (|CallParentFunction))