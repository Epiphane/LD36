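; A spike trap actor that kills the player on contact.
; On actor begin overlap it checks that the other actor is the first player's pawn, casts it to Explorer and calls Die.
; The GetSpikeZPosition graph holds only unused nodes that take the X component of the spike mesh's offset from the root, despite its name.
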(event Collision|EventActorBeginOverlap
  (params (OtherActor :type Actor%20Object%20Reference))
  (bind _returnvalue (Game|Player|GetPlayerPawn 0))
  ;[1 1 1] Activate Spikes
  (if (== OtherActor _returnvalue)
    (bind _asexplorer (Utilities|Casting|CastToExplorer _returnvalue))
    (Default|Die _asexplorer)))

(fn ConstructionScript)