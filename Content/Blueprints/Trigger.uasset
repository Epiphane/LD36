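; Pressure plate style trigger actor that reacts to the player pawn stepping on and off it.
; On begin overlap it nudges its Platform component down slightly, then calls Trigger on every element of the Triggers array.
; On end overlap it raises the Platform by the same offset, without notifying the Triggers.
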(event EventBeginPlay)

(event Collision|EventActorBeginOverlap
  (params (OtherActor :type Actor%20Object%20Reference))
  (if (== OtherActor (Game|Player|GetPlayerPawn 0))
    (Transformation|AddLocalOffset (Variables|Default|GetPlatform) "0, 0,-5.000000" false false)
    (for _array_element (Variables|Default|GetTriggers)
      (Default|Trigger _array_element))))

(event Collision|EventActorEndOverlap
  (params (OtherActor :type Actor%20Object%20Reference))
  (if (== OtherActor (Game|Player|GetPlayerPawn 0))
    (Transformation|AddLocalOffset (Variables|Default|GetPlatform) "0, 0,5.000000" false false)))

(fn ConstructionScript)