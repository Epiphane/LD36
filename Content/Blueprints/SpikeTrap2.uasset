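; Spike trap actor that kills the player's Explorer when the player pawn overlaps it.
; Overlap sets IsActivated, which nothing here resets, and calls Die on the Explorer.
; Tick moves five spike meshes at SpikeVelocity toward the active or inactive offset, correcting any overshoot.
; GetSpikeZPosition gates that movement, but its only expression is unconnected and reads relative X, not Z.
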(event Collision|EventActorBeginOverlap
  (params (OtherActor :type Actor%20Object%20Reference))
  (bind _returnvalue (Game|Player|GetPlayerPawn 0))
  ;[1 1 1] Activate Spikes
  (if (== OtherActor _returnvalue)
    (Variables|Default|SetIsActivated true)
    (bind _asexplorer (Utilities|Casting|CastToExplorer _returnvalue))
    (Default|Die _asexplorer)))

(event EventTick
  (params (DeltaSeconds :type Float%20%28single-precision%29))
  (bind _z (Utilities|GetSpikeZPosition))
  (bind _z_2 (Utilities|GetSpikeZPosition))
  (bind _spikevelocity (Variables|Default|GetSpikeVelocity))
  (bind _inactivespikeoffset (Variables|Default|GetInactiveSpikeOffset))
  (bind _activespikeoffset (Variables|Default|GetActiveSpikeOffset))
  (bind _returnvalue (- _activespikeoffset _z_2))
  (bind _returnvalue_2 (- _inactivespikeoffset _z))
  (bind _returnvalue_3 (* _spikevelocity DeltaSeconds))
  (bind _returnvalue_4 (Math|Vector|MakeVector 0.0 0.0 _returnvalue_3))
  ;[1 1 1] Animate Spikes
  (if (Variables|Default|GetIsActivated)
    ;;[1 1 1] Move Spikes up
    (if (< (Utilities|GetSpikeZPosition) (Variables|Default|GetActiveSpikeOffset))
      (Transformation|AddWorldOffset (Variables|Default|GetSpikeMesh) _returnvalue_4 false false)
      (if (< _returnvalue 0.0)
        (Transformation|AddWorldOffset (Variables|Default|GetSpikeMesh) (Math|Vector|MakeVector 0.0 0.0 _returnvalue) false false)))
    (else
      ;;[1 1 1] Move Spikes Down
      (if (> (Utilities|GetSpikeZPosition) (Variables|Default|GetInactiveSpikeOffset))
        (Transformation|AddWorldOffset (Variables|Default|GetSpikeMesh) (* _returnvalue_4 -1) false false)
        (if (> _returnvalue_2 0.0)
          (Transformation|AddWorldOffset (Variables|Default|GetSpikeMesh) (Math|Vector|MakeVector 0.0 0.0 _returnvalue_2) false false))))))

(fn ConstructionScript)