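; A falling platform actor that drops shortly after the player pawn touches it.
; Overlap with the player pawn sets a one-second TimeToFall countdown, which Tick decrements each frame.
; When the countdown runs out, Tick enables physics simulation on the Base component so the platform falls.
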(event EventBeginPlay)

(event EventTick
  (params (DeltaSeconds :type Float%20%28single-precision%29))
  ;[1 1 1] Drop Platform
  (if (> (Variables|Default|GetTimeToFall) 0.0)
    (Variables|Default|SetTimeToFall (- (Variables|Default|GetTimeToFall) DeltaSeconds))
    (if (<= (- (Variables|Default|GetTimeToFall) DeltaSeconds) 0.0)
      (Physics|SetSimulatePhysics (Variables|Default|GetBase) true))))

(event Collision|EventActorBeginOverlap
  (params (OtherActor :type Actor%20Object%20Reference))
  ;[1 1 1] Trigger
  (if (== OtherActor (Game|Player|GetPlayerPawn 0))
    (Variables|Default|SetTimeToFall 1.0)))

(fn ConstructionScript)