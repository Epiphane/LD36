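; StrobeLight is a light Blueprint that continually shifts between random colors as a strobe effect.
; Tick runs through a 0.1-second Delay, then picks a random RGB color and restarts the Strobe timeline.
; Each timeline update blends the light's current color toward that target, using the curve value as alpha.
; The Construction Script initializes the light to white.
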(event Collision|EventActorBeginOverlap
  (params (OtherActor :type Actor%20Object%20Reference)))

(event EventTick
  (params (DeltaSeconds :type Float%20%28single-precision%29))
  (bind _strobe_light (Variables|Default|GetStrobe%20Light))
  (Utilities|FlowControl|Delay 0.1)
  (bind _output_get (Variables|Default|SetNew%20light%20color (Math|Color|MakeColor (Math|Random|RandomFloatinRange 0.0 1.0) (Math|Random|RandomFloatinRange 0.0 1.0) (Math|Random|RandomFloatinRange 0.0 1.0))))
  (bind _strobe_curve (Timeline|Strobe PlayFromStart)
    (:Update
      (Rendering|Components|Light|SetLightColor _strobe_light (Math|Color|Lerp(LinearColor) (Rendering|Components|Light|GetLightColor _strobe_light) _output_get _strobe_curve) true))))

(fn ConstructionScript
  (Rendering|Components|Light|SetLightColor (Variables|Default|GetStrobe%20Light) "(R=1.000000,G=1.000000,B=1.000000,A=1.000000)" true))