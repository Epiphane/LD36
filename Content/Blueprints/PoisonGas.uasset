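; Poison gas hazard that drains the player Explorer's Breath while the player is in contact with it.
; Trigger extends the parent's behavior by activating the PPoisonGas effect.
; Overlap events track contact with player pawn 0, and Tick subtracts Strength per second from Breath during contact, with no check in this Blueprint that the gas has been triggered.
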(event EventTrigger
  (|CallParentFunction)
  (Components|Activation|SetActive (Variables|Default|GetP_PoisonGas) true false))

(event Collision|EventActorBeginOverlap
  (params (OtherActor :type Actor%20Object%20Reference))
  (if (== OtherActor (Game|Player|GetPlayerPawn 0))
    (Variables|Default|SetIsPlayerInContact true)))

(event Collision|EventActorEndOverlap
  (params (OtherActor :type Actor%20Object%20Reference))
  (if (== OtherActor (Game|Player|GetPlayerPawn 0))
    (Variables|Default|SetIsPlayerInContact false)))

(event EventTick
  (params (DeltaSeconds :type Float%20%28single-precision%29))
  (if (Variables|Default|GetIsPlayerInContact)
    (bind _asexplorer (Utilities|Casting|CastToExplorer (Game|Player|GetPlayerPawn 0)))
    (Variables|/Game/Blueprints/Explorer.Explorer_C|SetBreath _asexplorer (- (Variables|/Game/Blueprints/Explorer.Explorer_C|GetBreath _asexplorer) (* DeltaSeconds (Variables|Default|GetStrength))))))

(fn ConstructionScript
  (|CallParentFunction))