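; Movable actor that, once triggered, moves from its starting transform to a Destination transform over TransitionTime.
; BeginPlay stores the starting transform, and Trigger sets a one-way flag so the move runs only once.
; Tick accumulates clamped elapsed time and calls TransformObject, which linearly interpolates location, rotation and scale without sweeping.
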(event EventBeginPlay
  (Variables|Default|SetStart (Transformation|GetActorTransform)))

(event EventTrigger
  (if (not (Variables|Default|GetTriggered))
    (Variables|Default|SetTriggered true)))

(event EventTick
  (params (DeltaSeconds :type Float%20%28single-precision%29))
  (if (and (Variables|Default|GetTriggered) (< (Variables|Default|GetTimeElapsed) (Variables|Default|GetTransitionTime)))
    (Variables|Default|SetTimeElapsed (Math|Float|Min(Float) (+ DeltaSeconds (Variables|Default|GetTimeElapsed)) (Variables|Default|GetTransitionTime)))
    (CallFunction|TransformObject)))

(fn ConstructionScript
  (|CallParentFunction))

(fn TransformObject
  (Transformation|SetActorTransform (Math|Transform|Lerp(Transform) (Variables|Default|GetStart) (Variables|Default|GetDestination) (/ (Variables|Default|GetTimeElapsed) (Variables|Default|GetTransitionTime)))))